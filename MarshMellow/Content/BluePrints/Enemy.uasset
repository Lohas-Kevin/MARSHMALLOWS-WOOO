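; Enemy actor that registers itself with the level's PickUpController and dies when attacked.
; On BeginPlay it finds the first PickUpController in the world and passes it a self-reference through SendReferenceMessage.
; The AttackEnemy event prints that the named enemy is dead, then destroys the actor.
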(event EventBeginPlay
  (bind _outactors (Actor|GetAllActorsOfClass "/Game/BluePrints/PickUpController.PickUpController_C"))
  (Variables|Default|SetPickupManager (Utilities|Array|Get(acopy) _outactors))
  (Class|PickUpInterface|SendReference(Message) (Variables|Default|GetPickupManager) self))

(event Collision|EventActorBeginOverlap
  (params (OtherActor :type Actor%20Object%20Reference)))

(event EventTick
  (params (DeltaSeconds :type Float%20%28single-precision%29)))

(event EventAttackEnemy
  (params (Damege :type Float%20%28single-precision%29))
  (Development|PrintString (Utilities|String|Append (Utilities|GetObjectName self) " is dead now"))
  (Actor|DestroyActor))

(fn ConstructionScript)