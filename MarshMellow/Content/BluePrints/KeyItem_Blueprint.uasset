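; Key item pickup actor that registers itself with the level's PickUpController and can be picked up.
; On BeginPlay it finds the first PickUpController, sets its tag and sends that controller its object name with the "KeyItem" type.
; Its PickUpKeyItem event prints a debug string and destroys the actor.
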(event Custom|Send
  ;[1 1 1] Send the position message
  (Class|PickUpInterface|SendNameMessage(Message) (Variables|Default|GetPickUpController) (Utilities|GetObjectName self) "KeyItem"))

(event EventBeginPlay
  (bind _outactors (Actor|GetAllActorsOfClass "/Game/BluePrints/PickUpController.PickUpController_C"))
  (Variables|Default|SetPickUpController (Utilities|Array|Get(acopy) _outactors))
  (Variables|Default|SetTag "KeyItem_1")
  (CallFunction|Send))

(event Collision|EventActorBeginOverlap
  (params (OtherActor :type Actor%20Object%20Reference)))

(event EventTick
  (params (DeltaSeconds :type Float%20%28single-precision%29)))

(event EventPickUpKeyItem
  ;[1 1 1] This is for Key Item Pick up
  (Development|PrintString "Hello")
  (Actor|DestroyActor))

(fn ConstructionScript)