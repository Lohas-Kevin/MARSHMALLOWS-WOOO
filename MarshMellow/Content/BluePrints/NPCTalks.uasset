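; NPC dialogue actor that shows a click-through conversation of up to 21 text slots.
; StartDialogue enables input, adds a TextBox widget, shows the cursor and sets ActiveText to the first line.
; Left clicks advance DialogueIndex through a hard-coded nested branch chain, calling Leaving at an empty slot; a filled final slot has no exit.
; Leaving disables input, removes the widget, restores RevenantPlayerCharacter control and hides the cursor.
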(event Custom|Leaving
  (Input|DisableInput (Game|GetPlayerController 0))
  (Widget|RemovefromParent (stale Custom|Start%20Dialogue _returnvalue_2))
  (bind _asplayer_controller (Utilities|Casting|CastToPlayerController (Game|GetPlayerController 0)))
  (bind _outactors (Actor|GetAllActorsOfClass "/Game/BluePrints/RevenantPlayerCharacter.RevenantPlayerCharacter_C"))
  (for _array_element _outactors
    (Default|RestoreControl _array_element)
    (Variables|/Script/Engine.PlayerController|SetbShowMouseCursor _asplayer_controller false)))

(event Custom|Start%20Dialogue
  (bind _returnvalue (Game|GetPlayerController 0))
  (Input|EnableInput (Game|GetPlayerController 0))
  (bind _returnvalue_2 (UserInterface|CreateWidget "/Game/BluePrints/UI/TextBox.TextBox_C" _returnvalue))
  (UserInterface|Viewport|AddtoViewport _returnvalue_2 0)
  (bind _asplayer_controller (Utilities|Casting|CastToPlayerController _returnvalue))
  (Variables|/Script/Engine.PlayerController|SetbShowMouseCursor _asplayer_controller true)
  (Variables|Default|SetActiveText (Variables|Default|GetTextBox1))
  (Variables|Default|SetDialogueIndex 1))

(event Custom|UpdateText
  (if (Utilities|Enum|NotEqual(Enum) (Variables|Default|GetTextBox2) (Variables|Default|GetNull))
    (if (== (Variables|Default|GetDialogueIndex) 1)
      (Variables|Default|SetActiveText (Variables|Default|GetTextBox2))
      (Variables|Default|SetDialogueIndex 2)
      (elif (Utilities|Enum|NotEqual(Enum) (Variables|Default|GetTextBox3) (Variables|Default|GetNull))
        (if (== (Variables|Default|GetDialogueIndex) 2)
          (Variables|Default|SetActiveText (Variables|Default|GetTextBox3))
          (Variables|Default|SetDialogueIndex 3)
          (elif (Utilities|Enum|NotEqual(Enum) (Variables|Default|GetTextBox4) (Variables|Default|GetNull))
            (if (== (Variables|Default|GetDialogueIndex) 3)
              (Variables|Default|SetActiveText (Variables|Default|GetTextBox4))
              (Variables|Default|SetDialogueIndex 4)
              (elif (Utilities|Enum|NotEqual(Enum) (Variables|Default|GetTextBox5) (Variables|Default|GetNull))
                (if (== (Variables|Default|GetDialogueIndex) 4)
                  (Variables|Default|SetActiveText (Variables|Default|GetTextBox5))
                  (Variables|Default|SetDialogueIndex 5)
                  (elif (Utilities|Enum|NotEqual(Enum) (Variables|Default|GetTextBox6) (Variables|Default|GetNull))
                    (if (== (Variables|Default|GetDialogueIndex) 5)
                      (Variables|Default|SetActiveText (Variables|Default|GetTextBox6))
                      (Variables|Default|SetDialogueIndex 6)
                      (elif (Utilities|Enum|NotEqual(Enum) (Variables|Default|GetTextBox7) (Variables|Default|GetNull))
                        (if (== (Variables|Default|GetDialogueIndex) 6)
                          (Variables|Default|SetActiveText (Variables|Default|GetTextBox7))
                          (Variables|Default|SetDialogueIndex 7)
                          (elif (Utilities|Enum|NotEqual(Enum) (Variables|Default|GetTextBox8) (Variables|Default|GetNull))
                            (if (== (Variables|Default|GetDialogueIndex) 7)
                              (Variables|Default|SetActiveText (Variables|Default|GetTextBox8))
                              (Variables|Default|SetDialogueIndex 8)
                              (elif (Utilities|Enum|NotEqual(Enum) (Variables|Default|GetTextBox9) (Variables|Default|GetNull))
                                (if (== (Variables|Default|GetDialogueIndex) 8)
                                  (Variables|Default|SetActiveText (Variables|Default|GetTextBox9))
                                  (Variables|Default|SetDialogueIndex 9)
                                  (elif (Utilities|Enum|NotEqual(Enum) (Variables|Default|GetTextBox10) (Variables|Default|GetNull))
                                    (if (== (Variables|Default|GetDialogueIndex) 9)
                                      (Variables|Default|SetActiveText (Variables|Default|GetTextBox10))
                                      (Variables|Default|SetDialogueIndex 10)
                                      (elif (Utilities|Enum|NotEqual(Enum) (Variables|Default|GetTextBox11) (Variables|Default|GetNull))
                                        (if (== (Variables|Default|GetDialogueIndex) 10)
                                          (Variables|Default|SetActiveText (Variables|Default|GetTextBox11))
                                          (Variables|Default|SetDialogueIndex 11)
                                          (elif (Utilities|Enum|NotEqual(Enum) (Variables|Default|GetTextBox12) (Variables|Default|GetNull))
                                            (if (== (Variables|Default|GetDialogueIndex) 11)
                                              (Variables|Default|SetActiveText (Variables|Default|GetTextBox12))
                                              (Variables|Default|SetDialogueIndex 12)
                                              (elif (Utilities|Enum|NotEqual(Enum) (Variables|Default|GetTextBox13) (Variables|Default|GetNull))
                                                (if (== (Variables|Default|GetDialogueIndex) 12)
                                                  (Variables|Default|SetActiveText (Variables|Default|GetTextBox13))
                                                  (Variables|Default|SetDialogueIndex 13)
                                                  (elif (Utilities|Enum|NotEqual(Enum) (Variables|Default|GetTextBox14) (Variables|Default|GetNull))
                                                    (if (== (Variables|Default|GetDialogueIndex) 13)
                                                      (Variables|Default|SetActiveText (Variables|Default|GetTextBox14))
                                                      (Variables|Default|SetDialogueIndex 14)
                                                      (elif (Utilities|Enum|NotEqual(Enum) (Variables|Default|GetTextBox15) (Variables|Default|GetNull))
                                                        (if (== (Variables|Default|GetDialogueIndex) 14)
                                                          (Variables|Default|SetActiveText (Variables|Default|GetTextBox15))
                                                          (Variables|Default|SetDialogueIndex 15)
                                                          (elif (Utilities|Enum|NotEqual(Enum) (Variables|Default|GetTextBox16) (Variables|Default|GetNull))
                                                            (if (== (Variables|Default|GetDialogueIndex) 15)
                                                              (Variables|Default|SetActiveText (Variables|Default|GetTextBox16))
                                                              (Variables|Default|SetDialogueIndex 16)
                                                              (elif (Utilities|Enum|NotEqual(Enum) (Variables|Default|GetTextBox17) (Variables|Default|GetNull))
                                                                (if (== (Variables|Default|GetDialogueIndex) 16)
                                                                  (Variables|Default|SetActiveText (Variables|Default|GetTextBox17))
                                                                  (Variables|Default|SetDialogueIndex 17)
                                                                  (elif (Utilities|Enum|NotEqual(Enum) (Variables|Default|GetTextBox18) (Variables|Default|GetNull))
                                                                    (if (== (Variables|Default|GetDialogueIndex) 17)
                                                                      (Variables|Default|SetActiveText (Variables|Default|GetTextBox18))
                                                                      (Variables|Default|SetDialogueIndex 18)
                                                                      (elif (Utilities|Enum|NotEqual(Enum) (Variables|Default|GetTextBox19) (Variables|Default|GetNull))
                                                                        (if (== (Variables|Default|GetDialogueIndex) 18)
                                                                          (Variables|Default|SetActiveText (Variables|Default|GetTextBox19))
                                                                          (Variables|Default|SetDialogueIndex 19)
                                                                          (elif (Utilities|Enum|NotEqual(Enum) (Variables|Default|GetTextBox20) (Variables|Default|GetNull))
                                                                            (if (== (Variables|Default|GetDialogueIndex) 19)
                                                                              (Variables|Default|SetActiveText (Variables|Default|GetTextBox20))
                                                                              (Variables|Default|SetDialogueIndex 20)
                                                                              (elif (Utilities|Enum|NotEqual(Enum) (Variables|Default|GetTextBox21) (Variables|Default|GetNull))
                                                                                (if (== (Variables|Default|GetDialogueIndex) 20)
                                                                                  (Variables|Default|SetActiveText (Variables|Default|GetTextBox21))
                                                                                  (Variables|Default|SetDialogueIndex 21))
                                                                                (else
                                                                                  (CallFunction|Leaving))))
                                                                            (else
                                                                              (CallFunction|Leaving))))
                                                                        (else
                                                                          (CallFunction|Leaving))))
                                                                    (else
                                                                      (CallFunction|Leaving))))
                                                                (else
                                                                  (CallFunction|Leaving))))
                                                            (else
                                                              (CallFunction|Leaving))))
                                                        (else
                                                          (CallFunction|Leaving))))
                                                    (else
                                                      (CallFunction|Leaving))))
                                                (else
                                                  (CallFunction|Leaving))))
                                            (else
                                              (CallFunction|Leaving))))
                                        (else
                                          (CallFunction|Leaving))))
                                    (else
                                      (CallFunction|Leaving))))
                                (else
                                  (CallFunction|Leaving))))
                            (else
                              (CallFunction|Leaving))))
                        (else
                          (CallFunction|Leaving))))
                    (else
                      (CallFunction|Leaving))))
                (else
                  (CallFunction|Leaving))))
            (else
              (CallFunction|Leaving))))
        (else
          (CallFunction|Leaving))))
    (else
      (CallFunction|Leaving))))

(event EventBeginPlay)

(event Collision|EventActorBeginOverlap
  (params (OtherActor :type Actor%20Object%20Reference)))

(event EventTick
  (params (DeltaSeconds :type Float%20%28single-precision%29)))

(event Input|MouseEvents|LeftMouseButton
  (params (Key :type Key%20Structure))
  (:Pressed
    (CallFunction|UpdateText)))

(fn ConstructionScript)