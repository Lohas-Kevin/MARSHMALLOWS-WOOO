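; PickUpController is a message hub linking the main character with key items and, for battle testing, enemies.
; It records the character's reference and position, registers KeyItem and Receiver names in a set, and answers bag requests, removing matched key items.
; Enemies register into an array; after a short delay, a find request returns the nearest one and drops it from that array.
; Tick's loop over item positions does nothing.
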(event EventBeginPlay)

(event Collision|EventActorBeginOverlap
  (params (OtherActor :type Actor%20Object%20Reference)))

(event EventAddItemtoBagSend
  (params (ItemName :type String) (ItemType :type String))
  (bind _maincharacterreference (Variables|Default|GetMainCharacterReference))
  ;[1 1 1] This part is for pick up the Key Item
  (if (Utilities|Enum|Equal(Enum) ItemType "KeyItem_Blueprint_C")
    (if (Utilities|Set|Contains (Variables|Default|GetKeyItemSet) ItemName)
      (Class|PickUpInterface|AddItemtoBagReturn(Message) _maincharacterreference true)
      (bind _returnvalue (Utilities|Set|Remove (Variables|Default|GetKeyItemSet) ItemName))
      (if (not _returnvalue)
        (Development|PrintString "ERROR: failed to remove KeyItem From KeyItem Set"))
      (else
        (Class|PickUpInterface|AddItemtoBagReturn(Message) _maincharacterreference false)))
    (else
      (Class|PickUpInterface|AddItemtoBagReturn(Message) _maincharacterreference false))))

(event EventSendPositionMessage
  (params (Self%20Reference :type Actor%20Object%20Reference) (Position :type Vector :default "0, 0, 0") (Tag :type String))
  ;[1 1 1] Character Position
  (Variables|Default|SetMainCharacterReference Self%20Reference)
  (if (Utilities|Enum|Equal(Enum) Tag "MainCharacter")
    (Variables|Default|SetMainCharacterPosition Position)
    (else
      (Development|PrintString "ERROR: Failed to update Main Character's position "))))

(event EventTick
  (params (DeltaSeconds :type Float%20%28single-precision%29))
  ;[1 1 1] position chack part
  (bind _keys (Utilities|Map|Keys (Variables|Default|GetKeyItemPosition)))
  (for _array_element _keys
    _))

(event EventSendReference
  (params (Ref :type Actor%20Object%20Reference))
  ;[1 1 1] This part is for battle system testing
  (Utilities|Array|Add (Variables|Default|GetEnemy%20List) Ref))

(event EventSendNameMessage
  (params (Name :type String) (Type :type String))
  (bind _keyitemset (Variables|Default|GetKeyItemSet))
  ;[1 1 1] Item Tracking
  (if (Utilities|Enum|Equal(Enum) Type "KeyItem")
    (Utilities|Set|Add _keyitemset Name)
    (Development|PrintString Name false false)
    (elif (Utilities|Enum|Equal(Enum) Type "Receiver")
      (Utilities|Set|Add _keyitemset Name)
      (Development|PrintString Name false false)
      (else
        (Development|PrintString "ERROR: Wrong type detected in PickUpController")
        (Development|PrintString Type)
        (Development|PrintString Name)))))

(event EventFindEnemySend
  ;[1 1 1] This part is for battle system testing
  (Utilities|FlowControl|Delay 0.2)
  (bind (_enemy _newarray) (CallFunction|FindNearestEnemy (Variables|Default|GetEnemy%20List) (Variables|Default|GetMainCharacterReference)))
  (Variables|Default|SetEnemy%20List _newarray)
  (Class|PickUpInterface|FindEnemyReturn(Message) (Variables|Default|GetMainCharacterReference) _enemy))

(fn ConstructionScript)

(fn FindNearestEnemy
  (params (EnemySet :type Array%20of%20Actor%20Object%20References) (MainCharacter :type Actor%20Object%20Reference))
  (for _array_element EnemySet
    (if (< (LocalVariables|Getdistance) 0.0) ; check has distance been set or not
      (LocalVariables|Setdistance (Math|Float|Absolute(Float) (Math|Vector|VectorLength (- (Transformation|GetWorldLocation (Variables|/Script/Engine.Actor|GetRootComponent _array_element)) (Transformation|GetWorldLocation (Variables|/Script/Engine.Actor|GetRootComponent MainCharacter))))))
      (LocalVariables|SetTarget _array_element)
      (elif (< (Math|Float|Absolute(Float) (Math|Vector|VectorLength (- (Transformation|GetWorldLocation (Variables|/Script/Engine.Actor|GetRootComponent _array_element)) (Transformation|GetWorldLocation (Variables|/Script/Engine.Actor|GetRootComponent MainCharacter))))) (LocalVariables|Getdistance)) ; if set, check the distance,pick the smaller one
        (LocalVariables|Setdistance (Math|Float|Absolute(Float) (Math|Vector|VectorLength (- (Transformation|GetWorldLocation (Variables|/Script/Engine.Actor|GetRootComponent _array_element)) (Transformation|GetWorldLocation (Variables|/Script/Engine.Actor|GetRootComponent MainCharacter))))))
        (LocalVariables|SetTarget _array_element))))
  (bind _output_get (LocalVariables|SetLocalArrayCopy EnemySet))
  (bind _returnvalue (Utilities|Array|RemoveItem _output_get (LocalVariables|GetTarget)))
  (if _returnvalue
    (return (LocalVariables|GetTarget) (LocalVariables|GetLocalArrayCopy))
    (else
      (Development|PrintString "ERROR: Failed to remove enemy from array"))))